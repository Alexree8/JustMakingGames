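; MainMenuCharacter is the main menu character Blueprint, which launches the platformer and opens a dialogue.
; Pressing E calls LaunchPlatformer on the cached MainGameInstance, choosing Platformer or Platformer2 by its first-level completion flag.
; GoDialogue, while the first level is incomplete and no widget exists yet, shows a DialogueWD widget in UI-only input mode and clears the FirstLaunch flag.
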(event Custom|GoDialogue
  (if (not (Variables|/Game/BaseGameElements/MainGameInstance.MainGameInstance_C|GetFirstLevelComplite (Variables|Default|GetGame%20Instance%20Ref)))
    (Variables|Default|GetUI
      (:then)
      (:else
        (Utilities|IsValid (Variables|Default|GetUI)
          (:Is%20Valid
            _)
          (:Is%20Not%20Valid
            (bind _returnvalue (UserInterface|CreateWidget "/Game/UI/DialogueSystem/DialogueWD.DialogueWD_C" (Game|GetPlayerController 0)))
            (bind _output_get (Variables|Default|SetUI _returnvalue))))
        (UserInterface|Viewport|AddtoViewport _output_get 0)
        (Input|SetInputModeUIOnly (Game|GetPlayerController 0) _output_get "LockInFullscreen" false)
        (Variables|/Game/BaseGameElements/MainGameInstance.MainGameInstance_C|SetFirstLaunch (Variables|Default|GetGame%20Instance%20Ref) false)))))

(event EventBeginPlay
  (bind _asmain_game_instance (Utilities|Casting|CastToMainGameInstance (Game|GetGameInstance)))
  (Variables|Default|SetGame%20Instance%20Ref _asmain_game_instance))

(event Collision|EventActorBeginOverlap
  (params (OtherActor :type Actor%20Object%20Reference)))

(event Input|KeyboardEvents|E
  (params (Key :type Key%20Structure :default "None"))
  (bind _game_instance_ref (Variables|Default|GetGame%20Instance%20Ref))
  (:Pressed
    (if (Variables|/Game/BaseGameElements/MainGameInstance.MainGameInstance_C|GetFirstLevelComplite _game_instance_ref)
      (Default|LaunchPlatformer _game_instance_ref "/Game/Levels/Platformer2.Platformer2")
      (else
        (Default|LaunchPlatformer _game_instance_ref "/Game/Levels/Platformer.Platformer")))))

(fn ConstructionScript)