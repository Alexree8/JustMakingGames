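; FoldLeaf is an actor that works as a periodically folding platform, flipping its SMCube mesh between two orientations.
; Tick drives the cycle through a latent delay set by the Delay variable, then calls RotatePlatform, which waits one more second.
; RotatePlatform toggles IsRotate and snaps the cube's relative rotation to one of two fixed poses, with no interpolation.
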(event Custom|RotatePlatform
  (Utilities|FlowControl|Delay 1.0)
  (if (Variables|Default|GetIsRotate)
    (Variables|Default|SetIsRotate false)
    (Transformation|SetRelativeRotation (Variables|Default|GetSM_Cube) (Math|Rotator|MakeRotator 1.8e+02 -9e+01 0.0) false false)
    (else
      (Variables|Default|SetIsRotate true)
      (Transformation|SetRelativeRotation (Variables|Default|GetSM_Cube) "0.000000,0.000000,180.000000" false false))))

(event EventBeginPlay)

(event Collision|EventActorBeginOverlap
  (params (OtherActor :type Actor%20Object%20Reference)))

(event EventTick
  (params (DeltaSeconds :type Float%20%28single-precision%29))
  (Utilities|FlowControl|Delay (Variables|Default|GetDelay))
  (CallFunction|RotatePlatform))

(fn ConstructionScript)